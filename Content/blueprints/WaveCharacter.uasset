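; Player blob character that makes waves on the level's Piano actor and gets bounced upward by them.
; Releasing Space sets the Piano material's wave centre, calls GenWave and queues a delayed Impulse; excess queued waves briefly lock input.
; Left-stick Y gestures also trigger Impulse, which ignores its strength and timing inputs.
; Tick applies custom vertical-only gravity movement with height-based damping and pins camera height, while physical animation wobbles the blob mesh.
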(event `Key|SpaceBar`
  (params (Key :type "Key Structure" :default "AnyKey"))
  (:`Pressed`
    (if (`self.IsLockedSpace`)
      (if (> (- (`GameplayStatics.GetTimeSeconds`) (`self.IsLocked_Since`)) (`self.Locked_Time`))
        (set `self.IsLockedSpace` false)
        (set `self.space_ispressed` true))
      (else
        (set `self.space_ispressed` true)
        (`FMODBlueprintStatics.PlayEventAttached` "/Game/FMOD/Events/SoundFX/SFX_Wave.SFX_Wave" (`self.BlobCollision`) "None" (0.0 0.0 0.0) "KeepRelativeOffset"))))
  (:`Released`
    (set `self.space_ispressed` false)))

(event `InputAxis|LeftY`
  (params (AxisValue :type "Float (single-precision)"))
  (set `self.LY_Value` AxisValue)
  (if (`self.Is_Charging`)
    (if (`self.Is_Increasing`)
      (if (<= (`self.LY_Value`) 0.0)
        (if (not (>= (`self.LY_Value`) (`self.LY_Value_last`)))
          (set `self.Is_Increasing` false)
          (set `self.Is_Charging` false)
          (set `self.LY_ValueMax` (`self.LY_Value`))
          (set `self.Time_LastY` (`GameplayStatics.GetTimeSeconds`)))
        (set `self.LY_Value_last` (`self.LY_Value`))))
    (elif (<= (`self.LY_Value`) 0.0)
      (`self.Impulse` (`self.LY_ValueMax`) (- (`GameplayStatics.GetTimeSeconds`) (`self.Time_LastY`)))
      (set `self.Time_LastY` 0.0)
      (set `self.Is_Charging` true)
      (set `self.Is_Increasing` true)
      (set `self.LY_Value_last` 0.0)
      (set `self.LY_ValueMax` 0.0))))

(event `InputAxis|LeftX`
  (params (AxisValue :type "Float (single-precision)"))
  (set `self.LX_Value` AxisValue))

(event `self.ReceiveTick`
  (params (DeltaSeconds :type "Float (single-precision)"))
  (bind _camera (`self.Camera`))
  (bind _wave_timed (`self.Wave_Timed`))
  (bind (_returnvalue_x _returnvalue_y) (`KismetMathLibrary.BreakVector` (`SceneComponent.K2_GetComponentLocation` _camera)))
  (set `self.DeltaTime` DeltaSeconds)
  (`|ExecutionSequence`
    (:`then_0`
      (if (`self.space_ispressed`)
        (set `self.TotalTimeSpacePressed` (+ (`self.TotalTimeSpacePressed`) (`self.DeltaTime`)))
        (elif (!= (`self.TotalTimeSpacePressed`) 0.0)
          (set `self.TotalTimeSpacePressed` 0.0)
          (`self.Wave`)
          (`KismetArrayLibrary.Array_Add` (`self.Wave_Timed`) (`self.Wave_Retard`)))))
    (:`then_1`
      (`SceneComponent.K2_SetWorldLocation` _camera (`KismetMathLibrary.MakeVector` _returnvalue_x _returnvalue_y (`self.CameraZOffset`)) false false))
    (:`then_2`
      (`self.Apply_Physics`))
    (:`then_3`
      (if (> (`KismetArrayLibrary.Array_Length` _wave_timed) 2)
        (set `self.IsLockedSpace` true)
        (set `self.IsLocked_Since` (`GameplayStatics.GetTimeSeconds`)))
      (for (_array_element _array_index) _wave_timed
        (bind _returnvalue (- _array_element (`self.DeltaTime`)))
        (`KismetArrayLibrary.Array_Set` _wave_timed _array_index _returnvalue)
        (if (<= _returnvalue 0.0)
          (`self.Impulse` (`self.MaxSpaceValue`) (`self.TotalTimeSpacePressed`))
          (`KismetArrayLibrary.Array_Remove` (`self.Wave_Timed`) _array_index))))))

(event `self.ReceiveBeginPlay`
  (bind _bone (`self.bone`))
  (bind _blobphysical (`self.BlobPhysical`))
  (`|ExecutionSequence`
    (:`then_0`
      (`PrimitiveComponent.SetLinearDamping` (`self.BlobCollision`) 0.0))
    (:`then_1`
      (`PrimitiveComponent.SetPhysMaterialOverride` (`self.BlobCollision`) "/Game/PhysMaterial/SuperSlick.SuperSlick"))
    (:`then_2`
      (bind _outactors (`GameplayStatics.GetAllActorsOfClass` "/Game/piano.piano_C"))
      (set `self.PianoRef` (`KismetArrayLibrary.Array_Get` _outactors)))
    (:`then_3`
      (set `self.Locked_Time` (/ (`self.Wave_Retard`) 3.0)))
    (:`then_4`
      (`PhysicalAnimationComponent.SetSkeletalMeshComponent` _blobphysical (`self.blob`))
      (`PhysicalAnimationComponent.ApplyPhysicalAnimationSettingsBelow` _blobphysical _bone (make `PhysicalAnimationData` false 10000.0 10000.0 100.0 10.0 0.0 0.0) false)
      (`SkeletalMeshComponent.SetAllBodiesBelowSimulatePhysics` (`self.blob`) _bone true false))))

(event `apply`
  (params (OverlappedComponent :type "PrimitiveComponent Object Reference") (OtherActor :type "Actor Object Reference") (OtherComp :type "PrimitiveComponent Object Reference") (OtherBodyIndex :type Integer) (bFromSweep :type Boolean) (SweepResult :type "HitResult Structure (by ref)"))
  (cast `/Game/blueprints/WaveCharacter` OtherActor)
  (`self.Impulse` 0.0))

(fn `Apply_Physics`
  (bind (_returnvalue_x _returnvalue_y _returnvalue_z) (`KismetMathLibrary.BreakVector` (`self.K2_GetActorLocation`)))
  (bind (_returnvalue_x_2 _returnvalue_y_2) (`KismetMathLibrary.BreakVector` (`self.K2_GetActorLocation`)))
  (bind (_speed_x _speed_y _speed_z) (`KismetMathLibrary.BreakVector` (`self.Speed`)))
  (`|ExecutionSequence`
    (:`then_0`
      (bind _output_get (set `self.Speed` (+ (`self.Speed`) (* (`self.Gravity`) (* (`self.DeltaTime`) 5.0)))))
      (bind (_returnvalue_x_3 _returnvalue_y_3 _returnvalue_z_2) (`KismetMathLibrary.BreakVector` (+ _output_get (`self.K2_GetActorLocation`))))
      (bind (_sweephitresult _returnvalue) (`self.K2_SetActorLocation` (`KismetMathLibrary.MakeVector` _returnvalue_x_2 _returnvalue_y_2 _returnvalue_z_2) true))
      (if (not _returnvalue)
        (set `self.Speed` (0.0 0.0 0.0))))
    (:`then_1`
      (if (> _speed_z 0.0)
        (set `self.Speed` (/ (`self.Speed`) (`KismetMathLibrary.FClamp` (/ _returnvalue_z (`self.VerticalDivider`)) 1.0 (`self.MaxVerticalSpeed divider`))))))))

(fn `ColliderMove`
  (params (SphereCollider :type "SphereComponent Object Reference") (WaveTime :type "Float (double-precision)"))
  (`SceneComponent.K2_SetRelativeLocation` SphereCollider (`KismetMathLibrary.VLerp` (`SceneComponent.RelativeLocation` (`self.EndSphere`)) (`SceneComponent.RelativeLocation` (`self.Arrow`)) (/ WaveTime (* (`self.Wave_Retard`) 2.0))) false false))

(fn `Impulse`
  (params (MaxValue :type "Float (double-precision)") (Time :type "Float (double-precision)"))
  (bind (_returnvalue_x _returnvalue_y _returnvalue_z) (`KismetMathLibrary.BreakVector` (`self.K2_GetActorLocation`)))
  (bind _arrow (`self.Arrow`))
  (`|ExecutionSequence`
    (:`then_0`
      (if (not (> _returnvalue_z 400.0))
        (set `self.Speed` (+ (* (`KismetMathLibrary.Normal` (+ (`SceneComponent.GetForwardVector` _arrow) (* (`SceneComponent.GetUpVector` _arrow) 5.0))) (`self.JumpPower`)) (`self.Speed`)))))))

(fn `UserConstructionScript`
  (`|ExecutionSequence`
    (:`then_0`
      (`KismetArrayLibrary.Array_Clear` (`self.SphereCollision`)))
    (:`then_1`
      (for _ (range 4)
        (bind _returnvalue (`AddComponent|NODE_AddSphereComponent-1` :`RelativeTransform` (`KismetMathLibrary.MakeTransform` (0.0 0.0 0.0) (struct) (4.0 4.0 4.0))))
        (`KismetArrayLibrary.Array_Add` (`self.SphereCollision`) _returnvalue)
        (`SceneComponent.K2_SetRelativeLocation` _returnvalue (`SceneComponent.RelativeLocation` (`self.Arrow`)) false false)
        (`SceneComponent.SetVisibility` _returnvalue true true)
        (`PrimitiveComponent.IgnoreActorWhenMoving` _returnvalue (`self.PianoRef`) false)))))

(fn `Wave`
  (bind (_returnvalue_x _returnvalue_y _returnvalue_z) (`KismetMathLibrary.BreakVector` (`SceneComponent.K2_GetComponentLocation` (`self.Arrow`))))
  (`|ExecutionSequence`
    (:`then_2`
      (`MaterialInstanceDynamic.SetVectorParameterValue` (`/Game/piano.mioMateriale` (`self.PianoRef`)) "CentralPosition" (make `LinearColor` _returnvalue_x _returnvalue_y _returnvalue_z 1.0)))
    (:`then_3`
      (`/Game/piano.GenWave` (`self.PianoRef`)))))