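; Obstacle Blueprint for a game run by WaveGameMode, tied to that mode's obstacle velocity value.
; BeginPlay caches the game mode, and each Tick sets the actor's relative location to (ObstacleVel, 0, 0).
; The velocity is used as an absolute X position rather than added to the current one; an add-to-location calculation sits unused.
; Tick also prints the display name of Group, apparently for debugging.
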(event `self.ReceiveBeginPlay`
  (`|ExecutionSequence`
    (:`then_0`
      (bind _aswave_game_mode (cast `/Game/blueprints/WaveGameMode` (`GameplayStatics.GetGameMode`)))
      (set `self.gameModeRef` _aswave_game_mode))))

(event `self.ReceiveTick`
  (params (DeltaSeconds :type "Float (single-precision)"))
  (`self.K2_SetActorRelativeLocation` (`KismetMathLibrary.MakeVector` (`/Game/blueprints/WaveGameMode.obstacleVel` (`self.gameModeRef`))))
  (`KismetSystemLibrary.PrintString` (`KismetSystemLibrary.GetDisplayName` (`self.Group`))))

(fn `UserConstructionScript`)