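; Moving obstacle actor for a game run by WaveGameMode, where hitting it ends the game.
; It caches the game mode on BeginPlay and shifts itself along world X every Tick by the shared ObstacleVel, without sweep or delta-time scaling.
; A hit on its Box component plays Collisione and immediately quits the game.
; Logic subtracting PlayerLife exists but is disconnected.
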(event `self.ReceiveBeginPlay`
  (`|ExecutionSequence`
    (:`then_0`
      (bind _aswave_game_mode (cast `/Game/blueprints/WaveGameMode` (`GameplayStatics.GetGameMode`)))
      (set `self.gameModeRef` _aswave_game_mode))))

(event `self.ReceiveTick`
  (params (DeltaSeconds :type "Float (single-precision)"))
  (`self.K2_AddActorWorldOffset` (`KismetMathLibrary.MakeVector` (`/Game/blueprints/WaveGameMode.obstacleVel` (`self.gameModeRef`)))))

(event `self.Box.OnComponentHit`
  (params (HitComponent :type "PrimitiveComponent Object Reference") (OtherActor :type "Actor Object Reference") (OtherComp :type "PrimitiveComponent Object Reference") (NormalImpulse :type "Vector Structure") (Hit :type "HitResult Structure (by ref)"))
  (`FMODAudioComponent.Play` (`self.collisione`))
  (`KismetSystemLibrary.QuitGame` null "Quit"))

(fn `UserConstructionScript`)