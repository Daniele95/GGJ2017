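; WaveGameMode is the game mode for a wave game, handling player possession, life drain and obstacle scrolling.
; On BeginPlay it possesses the first WaveCharacter with player controller 0 and caches that controller as a WavePlayerController.
; Every Tick it lowers PlayerLife by a fixed amount and offsets all actors tagged "panner" along X by ObstacleVel, with neither step scaled by delta time.
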(event `self.ReceiveBeginPlay`
  (`|ExecutionSequence`
    (:`then_0`
      (bind _outactors (`GameplayStatics.GetAllActorsOfClass` "/Game/blueprints/WaveCharacter.WaveCharacter_C"))
      (`Controller.Possess` (`GameplayStatics.GetPlayerController` 0) (`KismetArrayLibrary.Array_Get` _outactors)))
    (:`then_1`
      (bind _aswave_player_controller (cast `/Game/blueprints/WavePlayerController` (`GameplayStatics.GetPlayerController` 0))
        (:`then`
          (set `self.PlayerConRef` _aswave_player_controller))
        (:`CastFailed`
          (`KismetSystemLibrary.PrintString` "Cast Fail"))))))

(event `self.ReceiveTick`
  (params (DeltaSeconds :type "Float (single-precision)"))
  (set `self.PlayerLife` (- (`self.PlayerLife`) 0.0001))
  (bind _outactors (`GameplayStatics.GetAllActorsWithTag` "panner"))
  (for _array_element _outactors
    (`self.K2_AddActorWorldOffset` _array_element (`KismetMathLibrary.MakeVector` (`self.ObstacleVel`)) false false)))

(fn `UserConstructionScript`)