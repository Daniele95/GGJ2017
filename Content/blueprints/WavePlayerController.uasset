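; WavePlayerController is a player controller that feeds a test UI with the wave character's charge state.
; On BeginPlay it creates the UI_Test widget, adds it to the viewport disabled and hidden, and caches the first WaveCharacter found.
; Each Tick it copies the character's LYValue into the widget and sets text labels for whether it is charging and whether it is increasing or decreasing.
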(event `self.ReceiveBeginPlay`
  (`|ExecutionSequence`
    (:`then_0`
      (bind _returnvalue (`|CreateWidget` "/Game/UI/UI_Test.UI_Test_C"))
      (`UserWidget.AddToViewport` _returnvalue 0)
      (bind _output_get (set `self.TestUi` _returnvalue))
      (`Widget.SetIsEnabled` _output_get false)
      (`Widget.SetVisibility` _output_get "Hidden"))
    (:`then_1`
      (bind _outactors (`GameplayStatics.GetAllActorsOfClass` "/Game/blueprints/WaveCharacter.WaveCharacter_C"))
      (set `self.CharacterRef` (`KismetArrayLibrary.Array_Get` _outactors)))))

(event `self.ReceiveTick`
  (params (DeltaSeconds :type "Float (single-precision)"))
  (bind _characterref (`self.CharacterRef`))
  (bind _testui (`self.TestUi`))
  (bind _ischarging (`/Game/UI/UI_Test.IsCharging` _testui))
  (bind _isincreasing (`/Game/UI/UI_Test.IsIncreasing` _testui))
  (set `/Game/UI/UI_Test.ValoreVisto` (`/Game/blueprints/WaveCharacter.LY_Value` (`self.CharacterRef`)) (`self.TestUi`))
  (`|ExecutionSequence`
    (:`then_0`
      (if (`/Game/blueprints/WaveCharacter.Is_Charging` _characterref)
        (`TextBlock.SetText` _ischarging "is charging")
        (else
          (`TextBlock.SetText` _ischarging "is not charging"))))
    (:`then_1`
      (if (`/Game/blueprints/WaveCharacter.Is_Increasing` _characterref)
        (`TextBlock.SetText` _isincreasing "is increasing")
        (else
          (`TextBlock.SetText` _isincreasing "is decreasing"))))))

(fn `UserConstructionScript`)